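; Game mode for the fantasy RTS that handles defeat when a friendly town hall is destroyed.
; On BeginPlay it caches all town halls and binds to each building component's destruction event.
; A Friendly destruction shows the lose widget.
; GetPlayerTownHall searches for the "Player" tag but indexes the town hall array with that tag's position, not the matching actor's.
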(event Custom|OnTownHallDestoryed
  (params (ClanAttit :type ETeamAttitude%20Enum :default "Friendly"))
  (if (Utilities|Enum|Equal(Enum) ClanAttit "Friendly")
    (CallFunction|LosetheGame)))

(event Custom|LoseTheGame
  (bind _returnvalue (UserInterface|CreateWidget "/Game/Fantasy_RTS/UI/Meanu/WBP_LOSE.WBP_LOSE_C"))
  (UserInterface|Viewport|AddtoViewport _returnvalue 0))

(event EventBeginPlay
  (bind _outactors (Actor|GetAllActorsOfClass "/Game/Fantasy_RTS/Buildings/BP_TownHall.BP_TownHall_C"))
  (bind _output_get (Variables|Default|SetTownHalls _outactors))
  (for _array_element _output_get
    (EventDispatchers|BindEventtoOnBuildingDestoryed (Actor|GetComponentbyClass _array_element "/Game/Fantasy_RTS/Core/Building/BP_BuildingCom.BP_BuildingCom_C") (delegate Custom|OnTownHallDestoryed))))

(event EventTick
  (params (DeltaSeconds :type Float%20%28single-precision%29)))

(fn ConstructionScript)

(fn GetPlayerTownHall
  (bind _array_element (Utilities|Array|ForEachLoopwithBreak (Variables|Default|GetTownHalls) :!label _label)
    (:LoopBody
      (if (>= (Utilities|Array|FindItem (Variables|/Script/Engine.Actor|GetTags _array_element) "Player") 0)
        (LocalVariables|SetIndex (Utilities|Array|FindItem (Variables|/Script/Engine.Actor|GetTags _array_element) "Player"))
        (goto _label Break)))
    (:Completed
      (return (Utilities|Array|Get(acopy) (Variables|Default|GetTownHalls) (LocalVariables|GetIndex))))))