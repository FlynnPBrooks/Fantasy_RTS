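; BP_ResourceComp is a component that represents a minable resource in the fantasy RTS, holding a resource type, a yield amount and a remaining mine count.
; GiveResource decrements the count, fires a gathered event, fires a depleted event once CanMine reports none left, then returns the type and amount.
; It does not check CanMine before giving, and its BeginPlay and Tick are empty.
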(event EventBeginPlay)

(event EventTick
  (params (DeltaSeconds :type Float%20%28single-precision%29)))

(fn GiveResource
  (Variables|Default|SetTimesitCanbeMined (- (Variables|Default|GetTimesitCanbeMined) 1))
  (Default|CallOnResourceGAthred)
  (Utilities|FlowControl|Sequence
    (:then_0
      (if (not (CallFunction|CanMine?))
        (Default|CallOnNoResscor)))
    (:then_1
      (return (Variables|Default|GetType) (Variables|Default|GetNumber_That_It_Gives)))))

(fn CanMine?
  (return (> (Variables|Default|GetTimesitCanbeMined) 0)))