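; BP_BuildingCom is a component that gives its owning building hit points and a health bar.
; On BeginPlay it adds a BP_HPWidgetCompo to the owner at a configured location and size, then binds to the owner's OnTakeAnyDamage.
; Damage lowers HP, clamped at zero, and pushes the HP ratio to the bar.
; At zero HP it calls the OnBuildingDestoryed dispatcher, with no guard against repeat calls on later hits.
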(event Custom|OnDamageTaken
  (params (DamagedActor :type Actor%20Object%20Reference) (Damage :type Float%20%28single-precision%29) (DamageType :type Damage%20Type%20Object%20Reference) (InstigatedBy :type Controller%20Object%20Reference) (DamageCauser :type Actor%20Object%20Reference))
  (Variables|Default|SetHP (Math|Float|Max(Float) (- (Variables|Default|GetHP) Damage) 0.0))
  (CallFunction|UpdateHP)
  (if (<= (Variables|Default|GetHP) 0.0)
    (Default|CallOnBuildingDestoryed)))

(event EventBeginPlay
  (Utilities|FlowControl|Sequence
    (:then_0
      (bind _returnvalue (Game|AddComponentbyClass (Components|GetOwner) "/Game/Fantasy_RTS/Core/Unit/BP_HPWidgetCompo.BP_HPWidgetCompo_C" false (Math|Transform|MakeTransform (Variables|HP|GetHPLocation) "0, 0, 0" "1.000000,1.000000,1.000000")))
      (Class|WidgetComponent|SetDrawSize _returnvalue (Variables|HP|GetSize))
      (CallFunction|UpdateHP))
    (:then_1
      (EventDispatchers|BindEventtoOnTakeAnyDamage (Components|GetOwner) (EventDispatchers|CreateEvent :!event Custom|OnDamageTaken)))))

(event EventTick
  (params (DeltaSeconds :type Float%20%28single-precision%29)))

(fn UpdateHP
  (bind _returnvalue (Components|GetOwner))
  (bind _returnvalue_2 (Actor|GetComponentbyClass _returnvalue "/Game/Fantasy_RTS/Core/Unit/BP_HPWidgetCompo.BP_HPWidgetCompo_C"))
  (Utilities|IsValid _returnvalue_2
    (:Is%20Valid
      (Default|UpdateHPBar _returnvalue_2 (/ (Variables|Default|GetHP) (Variables|Default|GetHPmax))))))