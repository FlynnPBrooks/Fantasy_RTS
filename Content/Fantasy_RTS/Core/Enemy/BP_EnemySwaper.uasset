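; BP_EnemySwaper is an enemy spawner that periodically creates waves of BP_Worker_Child_Clan2 units.
; On BeginPlay it starts a looping timer with a randomized initial delay, calling SpawnWave at the configured wave interval.
; Each wave passes a small random count to SpawnEnemy, which spawns units at random navigable points within the Sphere's radius, raised slightly and ignoring collisions.
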(event Custom|SpawnEnemy
  (params (Eenmiestospawn :type Integer))
  (for _index (range 0 Eenmiestospawn)
    (bind _randomlocation (Class|NavigationSystemV1|GetRandomLocationinNavigableRadius (Transformation|GetActorLocation) (Components|Sphere|GetScaledSphereRadius (Variables|Default|GetSphere)) 0 0))
    (Game|SpawnActorfromClass "/Game/Fantasy_RTS/Units/Clan2/BP_Worker_Child_Clan2.BP_Worker_Child_Clan2_C" (Math|Transform|MakeTransform (+ _randomlocation "0.000000,0.000000,100.000000") "0, 0, 0" "1.000000,1.000000,1.000000") "AlwaysSpawn" "MultiplyWithRoot" 0 0)))

(event Custom|SpawnWave
  (CallFunction|SpawnEnemy (Math|Random|RandomIntegerinRange 1 3)))

(event EventBeginPlay
  (bind _returnvalue (Utilities|Time|SetTimerbyEvent (delegate Custom|SpawnWave) (Variables|Default|GetTimeforWave) true false 2.0 2.0))
  (Variables|Default|SetSpawnTimer _returnvalue))

(event Collision|EventActorBeginOverlap
  (params (OtherActor :type Actor%20Object%20Reference)))

(event EventTick
  (params (DeltaSeconds :type Float%20%28single-precision%29)))

(fn ConstructionScript)