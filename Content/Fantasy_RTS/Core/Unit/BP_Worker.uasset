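; Worker unit for a fantasy RTS that moves on command, gathers resources, attacks targets and supports click selection when friendly.
; AI MoveTo drives orders, while BP_UnitComp holds the state that selects looping animations.
; Gathering waits out the mining time, delivers the load to the town hall and player controller, then repeats while the resource allows.
; Attacks apply damage on a looping timer, chasing targets that leave range.
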(event OnClicked(CapsuleComponent)
  (params (TouchedComponent :type Primitive%20Component%20Object%20Reference) (ButtonPressed :type Key%20Structure :default "None"))
  (if (Utilities|Enum|Equal(Enum) (Variables|/Game/Fantasy_RTS/Core/Unit/BP_UnitComp.BP_UnitComp_C|GetClanLoyalty (Variables|Default|GetBP_UnitComp)) "Friendly")
    (Class|BPISlection|SelectOnlyThisActor(Message) (Game|GetPlayerController 0) self)))

(event OnNewState(BP_UnitComp)
  (params (NewSate :type E_UnitState%20Enum :default "NewEnumerator0"))
  (Components|Animation|PlayAnimation (Variables|Character|GetMesh) (Utilities|Select :Index NewSate :NewEnumerator0 0 :NewEnumerator1 "/Game/Characters/DwarfGrunt/Anims/Idle_1_new.Idle_1_new" :NewEnumerator2 "/Game/Characters/DwarfGrunt/Anims/WalkFwd2.WalkFwd2" :NewEnumerator3 "/Game/Characters/DwarfGrunt/Anims/AnimMontageAttack_1_new.AnimMontageAttack_1_new" :NewEnumerator4 "/Game/Characters/DwarfGrunt/Anims/AnimMontageAttack_1_new.AnimMontageAttack_1_new") true))

(event Custom|GoToTownhallWithResource
  (params (ResourceRef :type Actor%20Object%20Reference))
  (Default|HadleNewStats (Variables|Default|GetBP_UnitComp) "NewEnumerator2")
  (bind _asgm_fantasy_rts (Utilities|Casting|CastToGM_Fantasy_RTS (Game|GetGameMode)))
  (AI|AIMoveTo self "0, 0, 0" (Default|GetPlayerTownHall _asgm_fantasy_rts) 2e+02 true
    (:OnSuccess
      (Default|HadleNewStats (Variables|Default|GetBP_UnitComp) "NewEnumerator1")
      (bind _aspc_fantasy_rts (Utilities|Casting|CastToPC_Fantasy_RTS (Game|GetPlayerController 0)))
      (Default|GetResources _aspc_fantasy_rts (Variables|Default|GetHasResource) (Variables|Default|GetNumberOfResource))
      (Variables|Default|SetHasResource "NewEnumerator0")
      (Variables|Default|SetNumberOfResource 0)
      (Utilities|IsValid ResourceRef
        (:Is%20Valid
          (CallFunction|RepeatMineing ResourceRef))))))

(event Custom|RepeatMineing
  (params (ResourceRef :type Actor%20Object%20Reference))
  (if (Default|CanMine? (Actor|GetComponentbyClass ResourceRef "/Game/Fantasy_RTS/Core/Resources/BP_ResourceComp.BP_ResourceComp_C"))
    (CallFunction|TakeThisResource ResourceRef)))

(event Custom|Attack
  (Variables|Default|GetTo%20Attack
    (:then
      (if (<= (Math|Vector|Distance(Vector) (Transformation|GetActorLocation (Variables|Default|GetTo%20Attack)) (Transformation|GetActorLocation)) (Variables|Default|GetRangeOfAttack))
        (Game|Damage|ApplyDamage (Variables|Default|GetTo%20Attack) (Variables|/Game/Fantasy_RTS/Core/Unit/BP_UnitComp.BP_UnitComp_C|GetDamage (Variables|Default|GetBP_UnitComp)) 0 0)
        (else
          (Utilities|Time|ClearandInvalidateTimerbyHandle (Variables|Default|GetAttacktimer))
          (if (Utilities|Enum|Equal(Enum) (Variables|/Game/Fantasy_RTS/Core/Unit/BP_UnitComp.BP_UnitComp_C|GetUnitstate (Variables|Default|GetBP_UnitComp)) "NewEnumerator4")
            (CallFunction|AttackThis (Variables|Default|GetTo%20Attack))))))
    (:else
      (CallFunction|StopAttack))))

(event Custom|StopAttack
  (Default|HadleNewStats (Variables|Default|GetBP_UnitComp) "NewEnumerator1")
  (Utilities|Time|ClearandInvalidateTimerbyHandle (Variables|Default|GetAttacktimer)))

(event EventMovetoThisPoint
  (params (Goal :type Vector :default "0, 0, 0"))
  (Default|HadleNewStats (Variables|Default|GetBP_UnitComp) "NewEnumerator2")
  (bind _movementresult (AI|AIMoveTo self Goal 0 5e+01 false)
    (:OnSuccess
      _)
    (:OnFail
      (switch Utilities|FlowControl|Switch|SwitchonEPathFollowingResult _movementresult
        (:Blocked
          _)
        (:OffPath
          _)
        (:Invalid
          _))))
  (Default|HadleNewStats (Variables|Default|GetBP_UnitComp) "NewEnumerator1"))

(event EventTakeThisResource
  (params (ResourceRef :type Actor%20Object%20Reference))
  (bind _returnvalue (Actor|GetComponentbyClass ResourceRef "/Game/Fantasy_RTS/Core/Resources/BP_ResourceComp.BP_ResourceComp_C"))
  (Default|HadleNewStats (Variables|Default|GetBP_UnitComp) "NewEnumerator2")
  (AI|AIMoveTo self "0, 0, 0" ResourceRef 2e+02 false
    (:OnSuccess
      (Transformation|SetActorRotation (Math|Rotator|MakeRotator 0.0 0.0 (.yaw (Math|Rotator|FindLookatRotation (Transformation|GetActorLocation) (Transformation|GetActorLocation ResourceRef)))))
      (if (and (Default|CanMine? _returnvalue) (Utilities|Enum|NotEqual(Enum) (Variables|Default|GetHasResource) (Variables|/Game/Fantasy_RTS/Core/Resources/BP_ResourceComp.BP_ResourceComp_C|GetType _returnvalue)))
        (Default|HadleNewStats (Variables|Default|GetBP_UnitComp) "NewEnumerator3")
        (Variables|Default|SetNumberOfResource 0)
        (Utilities|FlowControl|RetriggerableDelay (Variables|/Game/Fantasy_RTS/Core/Resources/BP_ResourceComp.BP_ResourceComp_C|GetTimeToMine _returnvalue))
        (if (Utilities|Enum|Equal(Enum) "NewEnumerator3" (Variables|/Game/Fantasy_RTS/Core/Unit/BP_UnitComp.BP_UnitComp_C|GetUnitstate (Variables|Default|GetBP_UnitComp)))
          (bind (_type _number_that_it_gives) (Default|GiveResource _returnvalue))
          (Variables|Default|SetHasResource _type)
          (Variables|Default|SetNumberOfResource _number_that_it_gives)
          (CallFunction|GotoTownhallwithResource ResourceRef))
        (elif (and (Utilities|Enum|Equal(Enum) (Variables|Default|GetHasResource) (Variables|/Game/Fantasy_RTS/Core/Resources/BP_ResourceComp.BP_ResourceComp_C|GetType _returnvalue)) (> (Variables|Default|GetNumberOfResource) 0))
          (CallFunction|GotoTownhallwithResource ResourceRef)
          (else
            (Default|HadleNewStats (Variables|Default|GetBP_UnitComp) "NewEnumerator1")))))))

(event EventInteractwithBuilding
  (params (BuildingRef :type Actor%20Object%20Reference))
  (bind _returnvalue (Actor|GetComponentbyClass BuildingRef "/Game/Fantasy_RTS/Core/Building/BP_BuildingCom.BP_BuildingCom_C"))
  (Utilities|IsValid _returnvalue
    (:Is%20Valid
      (if (> (Variables|Default|GetNumberOfResource) 0)
        (if (Utilities|Enum|Equal(Enum) (Variables|/Game/Fantasy_RTS/Core/Building/BP_BuildingCom.BP_BuildingCom_C|GetTypesOfBuilding _returnvalue) "NewEnumerator1")
          (CallFunction|GotoTownhallwithResource))))))

(event EventSelectThis
  (Default|ShowSelectionDecal (Variables|Default|GetBP_UnitComp)))

(event EventDeselectThis
  (Default|HideSelectionDecal (Variables|Default|GetBP_UnitComp)))

(event EventAttackThis
  (params (ToAttack :type Actor%20Object%20Reference))
  (Variables|Default|SetTo%20Attack ToAttack)
  (Default|HadleNewStats (Variables|Default|GetBP_UnitComp) "NewEnumerator2")
  (AI|AIMoveTo self "0, 0, 0" (Variables|Default|GetTo%20Attack) 2e+02 true
    (:OnSuccess
      (Variables|Default|SetRangeOfAttack (Math|Vector|Distance(Vector) (Transformation|GetActorLocation (Variables|Default|GetTo%20Attack)) (Transformation|GetActorLocation)))
      (Transformation|SetActorRotation (Math|Rotator|MakeRotator 0.0 0.0 (.yaw (Math|Rotator|FindLookatRotation (Transformation|GetActorLocation) (Transformation|GetActorLocation (Variables|Default|GetTo%20Attack))))))
      (Default|HadleNewStats (Variables|Default|GetBP_UnitComp) "NewEnumerator4")
      (bind _returnvalue (Utilities|Time|SetTimerbyEvent (delegate Custom|Attack) 1.0 true))
      (Variables|Default|SetAttacktimer _returnvalue))))

(fn ConstructionScript)