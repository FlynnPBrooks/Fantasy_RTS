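; BP_UnitSelection is the drag-selection volume for units in the Fantasy RTS.
; While resizing is active, Tick traces under the cursor and stretches a box between the actor's location and the hit point, with sphere components marking the cursor and midpoint.
; Box overlaps with BPI_Slection actors tell the player controller to select or, during resizing, deselect them.
; Start and end functions toggle resizing and box query collision.
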(event OnComponentBeginOverlap(Box)
  (params (OverlappedComponent :type Primitive%20Component%20Object%20Reference) (OtherActor :type Actor%20Object%20Reference) (OtherComp :type Primitive%20Component%20Object%20Reference) (OtherBodyIndex :type Integer) (bFromSweep :type Boolean) (SweepResult :type Hit%20Result%20Structure%20%28by%20ref%29))
  (if (Utilities|DoesObjectImplementInterface OtherActor "/Game/Fantasy_RTS/Core/Building/BPI_Slection.BPI_Slection_C")
    (Class|BPISlection|SelectThisActor(Message) (Game|GetPlayerController 0) OtherActor)))

(event OnComponentEndOverlap(Box)
  (params (OverlappedComponent :type Primitive%20Component%20Object%20Reference) (OtherActor :type Actor%20Object%20Reference) (OtherComp :type Primitive%20Component%20Object%20Reference) (OtherBodyIndex :type Integer))
  (if (and (Variables|Default|GetShouldResize) (Utilities|DoesObjectImplementInterface OtherActor "/Game/Fantasy_RTS/Core/Building/BPI_Slection.BPI_Slection_C"))
    (Class|BPISlection|DeselectThisActor(Message) (Game|GetPlayerController 0) OtherActor)))

(event EventBeginPlay)

(event Collision|EventActorBeginOverlap
  (params (OtherActor :type Actor%20Object%20Reference)))

(event EventTick
  (params (DeltaSeconds :type Float%20%28single-precision%29))
  (if (Variables|Default|GetShouldResize)
    (bind _aspc_fantasy_rts (Utilities|Casting|CastToPC_Fantasy_RTS (Game|GetPlayerController 0)))
    (Transformation|SetWorldLocation (Variables|Default|GetSphere) (.Location (Collision|BreakHitResult (.HitResult (Game|Player|GetHitResultUnderCursorbyChannel _aspc_fantasy_rts "TraceTypeQuery1" true)))) false false)
    (Variables|Default|SetEndMouseLocation (.Location (Collision|BreakHitResult (.HitResult (Game|Player|GetHitResultUnderCursorbyChannel _aspc_fantasy_rts "TraceTypeQuery1" true)))))
    (Transformation|SetWorldLocation (Variables|Default|GetBox) (Math|Vector|Lerp(Vector) (Transformation|GetActorLocation) (Variables|Default|GetEndMouseLocation) 0.5) false false)
    (Components|Box|SetBoxExtent (Variables|Default|GetBox) (Math|Vector|MakeVector (.x (/ (Math|Vector|VectorGetAbs (- (Transformation|GetActorLocation) (Variables|Default|GetEndMouseLocation))) 2.0)) (.y (/ (Math|Vector|VectorGetAbs (- (Transformation|GetActorLocation) (Variables|Default|GetEndMouseLocation))) 2.0)) 3e+02) true)))

(fn ConstructionScript)

(fn StartReizeing
  (Variables|Default|SetShouldResize true)
  (Collision|SetCollisionEnabled (Variables|Default|GetBox) "QueryOnly"))

(fn EndReizeing
  (Variables|Default|SetShouldResize false)
  (Collision|SetCollisionEnabled (Variables|Default|GetBox) "NoCollision"))