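; Player controller for the Fantasy RTS, handling camera movement, actor selection and unit move orders.
; WASD input moves the controlled pawn along its control yaw, falling back to screen-edge scroll scales computed from mouse position.
; Selection keeps one actor at a time, deselecting previous ones through BPI_Slection.
; Releasing MouseAction sends selected BPI_UnitActions actors to the cursor hit point and spawns a Niagara click indicator for each.
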(event Custom|AddActorSelectedList
  (params (SelectedActor :type Actor%20Object%20Reference))
  (CallFunction|DeselectedAllActors)
  (Utilities|Array|Add (Variables|Default|GetSelectedActors) SelectedActor))

(event Custom|DeselectedAllActors
  (for _array_element (Variables|Default|GetSelectedActors)
    (if (Utilities|DoesObjectImplementInterface _array_element "/Game/Fantasy_RTS/Core/Building/BPI_Slection.BPI_Slection_C")
      (Class|BPISlection|DeselectThis(Message) _array_element)))
  (Utilities|Array|Clear (Variables|Default|GetSelectedActors)))

(event EventBeginPlay)

(event EventTick
  (params (DeltaSeconds :type Float%20%28single-precision%29)))

(event Input|ActionEvents|InputActionMouseSelection
  (params (Key :type Key%20Structure :default "None")))

(event Input|ActionEvents|InputActionMouseAction
  (params (Key :type Key%20Structure :default "None"))
  (bind _hitresult (Game|Player|GetHitResultUnderCursorbyChannel "TraceTypeQuery1" true))
  (bind _location (Collision|BreakHitResult _hitresult))
  (:Released
    (if (Utilities|Array|IsNotEmpty (Variables|Default|GetSelectedActors))
      (for _array_element (Variables|Default|GetSelectedActors)
        (if (Utilities|DoesObjectImplementInterface _array_element "/Game/Fantasy_RTS/Core/Unit/BPI_UnitActions.BPI_UnitActions_C")
          (Class|BPIUnitActions|MovetoThisPoint(Message) _array_element _location)
          (Niagara|SpawnSystematLocation "/Game/Fantasy_RTS/Core/Player/NS_ClickInd.NS_ClickInd" _location))))))

(event Input|AxisEvents|InputAxisMoveForward
  (params (AxisValue :type Float%20%28single-precision%29))
  ;[1 1 1] Movement Camera and WASD
  (Pawn|Input|AddMovementInput (Pawn|GetControlledPawn) (Math|Vector|GetForwardVector (Math|Rotator|MakeRotator 0.0 0.0 (.yaw (Pawn|GetControlRotation (Pawn|GetControlledPawn) :!class /Script/Engine.Pawn)))) (Math|Float|SelectFloat AxisValue (Variables|Default|GetMouseForwardScale) (!= AxisValue 0.0)) false))

(event Input|AxisEvents|InputAxisMoveRight
  (params (AxisValue :type Float%20%28single-precision%29))
  ;[1 1 1] Movement Camera and WASD
  (Pawn|Input|AddMovementInput (Pawn|GetControlledPawn) (Math|Vector|GetRightVector (Math|Rotator|MakeRotator 0.0 0.0 (.yaw (Pawn|GetControlRotation (Pawn|GetControlledPawn) :!class /Script/Engine.Pawn)))) (Math|Float|SelectFloat AxisValue (Variables|Default|GetMouseRightScale) (!= AxisValue 0.0)) false))

(event Input|AxisEvents|InputAxisMouseMovement
  (params (AxisValue :type Float%20%28single-precision%29))
  (bind _locationy (Game|Player|GetMousePosition))
  (bind _returnvalue (Viewport|GetViewportSize))
  (bind _locationx (Game|Player|GetMousePosition))
  (bind _returnvalue_2 (Viewport|GetViewportSize))
  (bind _returnvalue_3 (/ _locationx (.x _returnvalue_2)))
  (bind _returnvalue_4 (/ _locationy (.y _returnvalue)))
  ;[1 1 1] Movement Camera and WASD
  (Variables|Default|SetMouseRightScale (Math|Float|SelectFloat -1.0 (Math|Float|SelectFloat 1.0 0.0 (> _returnvalue_3 (- 1.0 (Variables|Default|GetViewportEdgeThreshold)))) (< _returnvalue_3 (Variables|Default|GetViewportEdgeThreshold))))
  (Variables|Default|SetMouseForwardScale (Math|Float|SelectFloat 1.0 (Math|Float|SelectFloat -1.0 0.0 (> _returnvalue_4 (- 1.0 (Variables|Default|GetViewportEdgeThreshold)))) (< _returnvalue_4 (Variables|Default|GetViewportEdgeThreshold)))))

(fn ConstructionScript)